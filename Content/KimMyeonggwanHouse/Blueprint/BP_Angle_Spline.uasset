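; Spline-driven wall builder that lays segment meshes, doors and corner pieces along a spline at construction time.
; Each span is split into stretched spline meshes sized from the base mesh, with A/B/C variants chosen by segment index.
; Listed points get instanced doors with gaps left for them; others can get instanced corners on CurveClamped points.
; Optional line traces snap heights to surfaces, and terracing levels segments; debug index drawing is disconnected.
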(event `self.ReceiveBeginPlay`
  ;[1 1 1] 포인트 및 리턴 포인트 번호(INDEX) DRAW DEBUG
)

(fn `Function Point B`
  (params (TargetArray :type "Array of Integer (by ref)"))
  (if (`KismetArrayLibrary.Array_Contains` TargetArray (`self.Point Index`))
    (`StaticMeshComponent.SetStaticMesh` (`self.Point SM Var`) (select `int` (`self.Select B Point`) :`0` (`self.0 Point Mesh`) :`1` (`self.1 Point Mesh`)))))

(fn `FunctionPoint C`
  (params (TargetArray :type "Array of Integer (by ref)"))
  (if (`KismetArrayLibrary.Array_Contains` TargetArray (`self.Point Index`))
    (`StaticMeshComponent.SetStaticMesh` (`self.Point SM Var`) (select `int` (`self.Select C Point`) :`0` (`self.0 Point Mesh`) :`1` (`self.1 Point Mesh`)))))

(fn `Line Trace `
  (params (InVec :type "Vector Structure"))
  (returns (OutHit_Location_Z :type "Float (double-precision)"))
  (bind _x (.x InVec))
  (bind _y (.y InVec))
  (bind _z (.z InVec))
  (bind _outhit (`KismetSystemLibrary.LineTraceSingle` (`KismetMathLibrary.MakeVector` _x _y (+ _z (`self.Trace Start`))) (`KismetMathLibrary.MakeVector` _x _y (- _z (`self.Trace End`))) (`self.Trace Channel`) false (`self.Actors to Ignore`) "ForDuration"))
  (return (.z (`.Location` (`GameplayStatics.BreakHitResult` _outhit)))))

(fn `MeshCenterOnPos`
  (params (InstanceMesh :type "StaticMeshComponent Object Reference") (Location :type "Vector Structure"))
  (returns (CenterLocation :type "Vector Structure"))
  (bind (_min _max) (`StaticMeshComponent.GetLocalBounds` InstanceMesh))
  (return (`KismetMathLibrary.MakeVector` (.x (- (- Location _min) (/ (- _max _min) (2.0 2.0 2.0)))) (.y (- (- Location _min) (/ (- _max _min) (2.0 2.0 2.0)))))))

(fn `UserConstructionScript`
  (locals (GLDAS_Start :type "Vector Structure" :default (0.0 0.0 0.0)) (GLDAS_End :type "Vector Structure" :default (0.0 0.0 0.0)) (GTDAS_Start :type "Vector Structure" :default (0.0 0.0 0.0)) (GTDAS_End :type "Vector Structure" :default (0.0 0.0 0.0)))
  (bind _spline (`self.Spline`))
  (bind _current_spline_index (`self.Current Spline Index`))
  (bind _snap_to_actor (`self.Snap to Actor`))
  (bind _mesh_margin (`self.Mesh Margin`))
  (bind _spline_2 (`self.Spline`))
  (bind _doorism (`self.DoorISM`))
  (bind _doormeshcenteronspline (`self.DoorMeshCenterOnSpline`))
  (bind _current_spline_index_2 (`self.Current Spline Index`))
  (bind _spline_3 (`self.Spline`))
  (bind _closedloopspline (`self.ClosedLoopSpline`))
  (bind _point_index (`self.Point Index`))
  (bind _spline_4 (`self.Spline`))
  (bind _spline_5 (`self.Spline`))
  (bind _returnvalue (`KismetArrayLibrary.Array_Contains` (`self.DoorSegmentPoint`) _current_spline_index_2))
  (bind _returnvalue_2 (`SplineComponent.GetDistanceAlongSplineAtSplinePoint` _spline _current_spline_index_2))
  (bind _returnvalue_3 (`SplineComponent.GetTransformAtSplinePoint` _spline_2 _current_spline_index "Local" false))
  (bind _returnvalue_4 (+ _current_spline_index_2 1))
  (`|ExecutionSequence`
    (:`then_0`
      ;[1 1 1] BaseMeshLengh
      (bind _base_segment_mesh (`self.Base Segment Mesh`)
        (:`then`
          (bind (_returnvalue_min _returnvalue_max) (break `Box` (`StaticMesh.GetBoundingBox` _base_segment_mesh)))
          (bind _returnvalue_x (`KismetMathLibrary.BreakVector` (- _returnvalue_max _returnvalue_min)))
          (set `self.MeshLength` _returnvalue_x))
        (:`else`)))
    (:`then_1`
      (`|ExecutionSequence`
        (:`then_0`
          (if _closedloopspline
            (`SplineComponent.SetClosedLoop` _spline_3 _closedloopspline true)
            (`SplineComponent.AddSplinePointAtIndex` _spline_3 (`SplineComponent.GetLocationAtSplinePoint` _spline_3 0 "Local") (`SplineComponent.GetNumberOfSplinePoints` _spline_3) "Local" true)))
        (:`then_1`
          (bind _doormesh (`self.DoorMesh`)
            (:`then`
              (bind _returnvalue_5 (`AddComponent|NODE_AddInstancedStaticMeshComponent-1`))
              (bind _output_get (set `self.DoorISM` _returnvalue_5))
              (`StaticMeshComponent.SetStaticMesh` _output_get _doormesh))
            (:`else`)))
        (:`then_2`
          (bind _doormesh_2 (`self.DoorMesh`)
            (:`then`
              (bind (_returnvalue_min_2 _returnvalue_max_2) (break `Box` (`StaticMesh.GetBoundingBox` _doormesh_2)))
              (bind _returnvalue_x_2 (`KismetMathLibrary.BreakVector` (- _returnvalue_max_2 _returnvalue_min_2)))
              (set `self.DoorMeshLength` (/ (- _returnvalue_x_2 (`self.DoorMeshMargin`)) 2.0)))
            (:`else`)))))
    (:`then_2`
      ;[1 1 1] SanapLandscape Only
      (if (`self.Snap to only Landscape`)
        (set `self.Trace Channel` "TraceTypeQuery3")
        (else
          (set `self.Trace Channel` "TraceTypeQuery1"))))
    (:`then_3`
      ;[1 1 1] CorrnerMesh
      (bind _base_point_mesh (`self.Base Point Mesh`)
        (:`then`
          (bind _returnvalue_6 (`AddComponent|NODE_AddInstancedStaticMeshComponent-0`))
          (bind _output_get_2 (set `self.ConnerISM` _returnvalue_6))
          (`StaticMeshComponent.SetStaticMesh` _output_get_2 _base_point_mesh))
        (:`else`)))
    (:`then_4`
      ;[1 1 1] Comment
      (for _index (range (+ (- (`SplineComponent.GetNumberOfSplinePoints` (`self.Spline`)) 2) 1))
        (set `self.Current Spline Index` _index)
        (`|ExecutionSequence`
          (:`then_0`
            ;[1 1 1] 포인트와 포인트사이의 길이 계산 및 배치 가능한 메시 개수 설정
            (bind _output_get_3 (set `self.Currnet Spline Distance` (`KismetMathLibrary.SelectFloat` (+ (`self.DoorMeshLength`) _returnvalue_2) _returnvalue_2 _returnvalue)))
            (bind _returnvalue_7 (- (`SplineComponent.GetDistanceAlongSplineAtSplinePoint` _spline _returnvalue_4) _output_get_3))
            (bind _output_get_4 (set `self.Currnet Spline Lenght` (`KismetMathLibrary.SelectFloat` (- _returnvalue_7 (`self.DoorMeshLength`)) _returnvalue_7 (`KismetArrayLibrary.Array_Contains` (`self.DoorSegmentPoint`) _returnvalue_4))))
            (bind _output_get_5 (set `self.Currnet Spline Num Mesh` (`KismetMathLibrary.FTrunc` (/ _output_get_4 (`self.MeshLength`)))))
            ;[1 1 1] 배치할 메시 길이 설정
            (if (not (> _output_get_5 0.0))
              (set `self.Currnet Spline Num Mesh` 1))
            (bind _output_get_6 (set `self.Stretched Mesh Length` (/ (`self.Currnet Spline Lenght`) (`self.Currnet Spline Num Mesh`))))
            (if (not (< _output_get_6 (* (`self.MeshLength`) 1.5)))
              (set `self.Stretched Mesh Length` (/ (`self.Stretched Mesh Length`) 2.0))
              (set `self.Currnet Spline Num Mesh` (* (`self.Currnet Spline Num Mesh`) 2)))
            (for _index_2 (range (`self.Currnet Spline Num Mesh`))
              ;[1 1 1] Door Point Index
              (`/Engine/EditorBlueprintResources/StandardMacros.IncrementInt` (`self.Point Index`)
                (:`  `
                  (`|ExecutionSequence`
                    (:`then_0`
                      ;[1 1 1] Start Position
                      (if (`self.Snap to Actor`)
                        (`|ExecutionSequence`
                          (:`then_0`
                            (bind _retrun (`self.CalcDistance2Mesh` _index_2 (* _mesh_margin -1.0)))
                            (bind _outhit_location_z (`self.Line Trace ` (`SplineComponent.GetLocationAtDistanceAlongSpline` _spline_5 _retrun "World"))))
                          (:`then_1`
                            (bind _retrun_2 (`self.CalcDistance2Mesh` (+ _index_2 1) _mesh_margin))
                            ;[1 1 1] End Position
                            (bind _outhit_location_z_2 (`self.Line Trace ` (`SplineComponent.GetLocationAtDistanceAlongSpline` _spline_4 _retrun_2 "World")))))))
                    (:`then_2`
                      (bind _returnvalue_8 (`AddComponent|NODE_AddSplineMeshComponent-1` :`RelativeTransform` (`KismetMathLibrary.MakeTransform` (`KismetMathLibrary.MakeVector` 0.0 0.0 (`self.Base Segment Height`)))))
                      (bind _returnvalue_9 (- _retrun 1.0))
                      (bind (_returnvalue_x_3 _returnvalue_y _returnvalue_z) (`KismetMathLibrary.BreakVector` (`SplineComponent.GetLocationAtDistanceAlongSpline` _spline_5 _returnvalue_9 "Local")))
                      (bind _returnvalue_10 (+ _retrun_2 1.0))
                      (bind (_returnvalue_x_4 _returnvalue_y_2 _returnvalue_z_2) (`KismetMathLibrary.BreakVector` (`SplineComponent.GetLocationAtDistanceAlongSpline` _spline_4 _returnvalue_10 "Local")))
                      (bind (_out_start_position _out_end_position) (`self.Make Segment Position` (`KismetMathLibrary.MakeVector` _returnvalue_x_3 _returnvalue_y (`KismetMathLibrary.SelectFloat` _outhit_location_z _returnvalue_z (`self.Snap to Actor`))) (`KismetMathLibrary.MakeVector` _returnvalue_x_4 _returnvalue_y_2 (`KismetMathLibrary.SelectFloat` _outhit_location_z_2 _returnvalue_z_2 (`self.Snap to Actor`)))))
                      (`SplineMeshComponent.SetStartAndEnd` _returnvalue_8 _out_start_position (`self.Make Tangent` (`SplineComponent.GetTangentAtDistanceAlongSpline` _spline_5 _returnvalue_9 "Local")) _out_end_position (`self.Make Tangent` (`SplineComponent.GetTangentAtDistanceAlongSpline` _spline_4 _returnvalue_10 "Local")) true)
                      (`StaticMeshComponent.SetStaticMesh` _returnvalue_8 (select `int` (`KismetMathLibrary.SelectInt` 1 (`KismetMathLibrary.SelectInt` 2 (`KismetMathLibrary.SelectInt` 3 0 (`KismetArrayLibrary.Array_Contains` (`self.C Segment Point`) _point_index)) (`KismetArrayLibrary.Array_Contains` (`self.B Segment Point`) _point_index)) (`KismetArrayLibrary.Array_Contains` (`self.A Segment Point`) _point_index)) :`0` (`self.Base Segment Mesh`) :`1` (`self.A SegmentMesh`) :`2` (`self.B SegmentMesh`) :`3` (`self.C SegmentMesh`)))
                      (`SceneComponent.K2_AttachToComponent` _returnvalue_8 (`self.Spline`) "None" "KeepRelative" "KeepRelative" "KeepRelative" true)))))))
          (:`then_1`
            ;[1 1 1] Original Spline index Location
            (if _snap_to_actor :!label _label
              (bind _outhit_location_z_3 (`self.Line Trace ` (`SplineComponent.GetLocationAtSplinePoint` _spline_2 _current_spline_index "World"))))
            (if _returnvalue
              ;[1 1 1] DoorMesh
              (if _doormeshcenteronspline
                (bind _returnvalue_11 (`KismetMathLibrary.SelectFloat` _outhit_location_z_3 (.z (.location _returnvalue_3)) _snap_to_actor))
                (bind _returnvalue_12 (`KismetMathLibrary.MakeVector` (.x (.location _returnvalue_3)) (.y (.location _returnvalue_3)) _returnvalue_11))
                (bind _centerlocation (`self.MeshCenterOnPos` _doorism _returnvalue_12)))
              (bind (_returnvalue_x_5 _returnvalue_y_3) (`KismetMathLibrary.BreakVector` (`KismetMathLibrary.SelectVector` _centerlocation _returnvalue_12 _doormeshcenteronspline)))
              (`InstancedStaticMeshComponent.AddInstance` _doorism (`KismetMathLibrary.MakeTransform` (+ (`self.DoorMeshOffset`) (`KismetMathLibrary.MakeVector` _returnvalue_x_5 _returnvalue_y_3 _returnvalue_11)) (.rotation _returnvalue_3) (.scale _returnvalue_3)) false)
              (else
                ;[1 1 1] ConnerMesh
                (if (and (`|EnumEquality` (`SplineComponent.GetSplinePointType` _spline_2 _current_spline_index) "CurveClamped") (`self.Couner Mesh Use`))
                  (`InstancedStaticMeshComponent.AddInstance` (`self.ConnerISM`) (`KismetMathLibrary.MakeTransform` _returnvalue_12 (`KismetMathLibrary.MakeRotator` 0.0) (.scale _returnvalue_3)) false)))))))
      (`/Engine/EditorBlueprintResources/StandardMacros.IncrementInt` (`self.Current Spline Index`)
        (:`  `
          (goto _label))))))